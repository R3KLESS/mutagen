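; Player controller for the login screen, which it sets up on BeginPlay only on the remote (non-authority) side.
; It matches the game resolution to the desktop through GameUserSettings, then applies Windowed mode, although an inline note says fullscreen.
; It creates the MutagenLogin_WB widget, stores it on mutagenGameInstance for later use, adds it to the viewport and enables game-and-UI input with a visible, locked cursor.
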(event EventBeginPlay
  (Networking|SwitchHasAuthority
    (:Remote
      (CallFunction|SetupLoginScreen))))

(fn ConstructionScript)

(fn SetupLoginScreen
  (CallFunction|SetupScreenResolution)
  (CallFunction|CreateLoginWidget))

(fn SetupScreenResolution
  ;[0 0.7605 1] gets the users desktop screen resolution and sets the games resolution to be the same
  (bind _returnvalue (Settings|GetGameUserSettings))
  (Class|GameUserSettings|SetScreenResolution _returnvalue (Class|GameUserSettings|GetDesktopResolution _returnvalue))
  (Class|GameUserSettings|ApplyResolutionSettings _returnvalue false)
  ;[0 0.7605 1] changes the screen mode to be fullscreen
  (Class|GameUserSettings|SetFullscreenMode _returnvalue "Windowed")
  (Class|GameUserSettings|ApplySettings _returnvalue false))

(fn CreateLoginWidget
  ;[0 0.7605 1] 1) creates the login widget
  ; 2) stores a reference to the loginwidget inside the gameinstance class to be used later
  ; 3) adds the widget to the screen
  (bind _returnvalue (UserInterface|CreateWidget "/Game/Blueprints/widgets/mutagenLogin_WB.mutagenLogin_WB_C" self))
  (bind _asmutagen_game_instance (Utilities|Casting|CastTomutagenGameInstance (Game|GetGameInstance)))
  (Variables|/Script/mutagen.mutagenGameInstance|SetloginWidgetRef _asmutagen_game_instance _returnvalue)
  (UserInterface|Viewport|AddtoViewport _returnvalue 0)
  (Input|SetInputModeGameandUI self 0 "LockAlways" false)
  (Variables|Default|SetbShowMouseCursor true))