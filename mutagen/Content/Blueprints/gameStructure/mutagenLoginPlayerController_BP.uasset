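; Player controller for the login screen, which sets up display settings and the login widget on remote clients at BeginPlay.
; Setup matches the game resolution to the desktop, applies Windowed mode despite a comment saying fullscreen, then adds MutagenLogin_WB to the viewport with game-only input.
; Pressing the enterKeyPress action reveals the widget's login panel, switches input to game-and-UI with mouse lock, and shows the cursor.
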(event EventBeginPlay
  (Networking|SwitchHasAuthority
    (:Remote
      (CallFunction|SetupLoginScreen))))

(event Input|ActionEvents|InputActionenterKeyPress
  (params (Key :type Key%20Structure :default "AnyKey"))
  (:Pressed
    (CallFunction|ShowLoginScreen)))

(fn ConstructionScript)

(fn SetupLoginScreen
  (CallFunction|SetupScreenResolution)
  (CallFunction|CreateLoginWidget))

(fn SetupScreenResolution
  ;[0 0.7605 1] gets the users desktop screen resolution and sets the games resolution to be the same
  (bind _returnvalue (Settings|GetGameUserSettings))
  (Class|GameUserSettings|SetScreenResolution _returnvalue (Class|GameUserSettings|GetDesktopResolution _returnvalue))
  (Class|GameUserSettings|ApplyResolutionSettings _returnvalue false)
  ;[0 0.7605 1] changes the screen mode to be fullscreen
  (Class|GameUserSettings|SetFullscreenMode _returnvalue "Windowed")
  (Class|GameUserSettings|ApplySettings _returnvalue false))

(fn CreateLoginWidget
  ;[0 0.1776 1] 1) creates the login widget
  ; 2) stores a reference to the loginwidget to be used later
  ; 3) adds the widget to the screen
  ; 4) sets the input mode to game only
  (bind _returnvalue (UserInterface|CreateWidget "/Game/Blueprints/widgets/mutagenLogin_WB.mutagenLogin_WB_C" self))
  (bind _output_get (Variables|Default|SetloginWidgetReference _returnvalue))
  (UserInterface|Viewport|AddtoViewport _output_get 0)
  (Input|SetInputModeGameOnly self))

(fn ShowLoginScreen
  (Default|ShowLoginPanel (Variables|Default|GetloginWidgetReference))
  (Input|SetInputModeGameandUI self 0 "LockAlways" false)
  (Variables|Default|SetbShowMouseCursor true))