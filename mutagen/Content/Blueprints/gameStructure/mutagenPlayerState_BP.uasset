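; Player state that handles account registration, activation, login and character checks against PHP scripts through VaRest JSON POST requests.
; SendRequestEvent builds each request by type from the login widget, cached a second after BeginPlay, and OnRequestComplete routes responses back to its messages and panels.
; Registration generates a random account ID client-side.
; Login stores session key and user ID, then requests a character check, whose response handler is an unconnected stub.
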(event Custom|SendRequestEvent
  (params (Request%20Type :type RequestType%20Enum))
  (Variables|VaRest|SetSentRequest (Class|VaRestRequestJSON|ConstructRequestExt "POST" "json"))
  (bind _output_get (Variables|VaRest|SetRequestType Request%20Type))
  (switch Utilities|FlowControl|Switch|SwitchonRequestType _output_get
    (:NewEnumerator0
      (CallFunction|CreateRegistrationRequest))
    (:NewEnumerator1
      (CallFunction|CreateActivationRequest))
    (:NewEnumerator2
      (CallFunction|CreateLoginRequest))
    (:NewEnumerator3
      (CallFunction|CreateCheckforCharactersRequest)))
  (EventDispatchers|BindEventtoOnRequestComplete (Variables|VaRest|GetSentRequest) (delegate Custom|OnRequestComplete)))

(event Custom|OnRequestComplete
  (params (Request :type Va%20Rest%20Request%20JSON%20Object%20Reference))
  (switch Utilities|FlowControl|Switch|SwitchonRequestType (Variables|VaRest|GetRequestType)
    (:NewEnumerator0
      (CallFunction|OnResponceRegistration))
    (:NewEnumerator1
      (CallFunction|OnResponceActivation))
    (:NewEnumerator2
      (CallFunction|OnResponceLogin))))

(event EventBeginPlay
  ;[0 0.1364 1] When play begins call the SetupLoginWidgetRef function
  ; so that we can get a reference to the login widget that was created
  (Utilities|Time|SetTimerbyFunctionName 0 "SetupLoginWidgetRef" 1.0))

(fn ConstructionScript)

(fn CreateRegistrationRequest
  ;[0 0.1364 1] Set all the varest String Fields that was entered on the registration page
  (bind _returnvalue (Class|VaRestRequestJSON|GetRequestObject (Variables|VaRest|GetSentRequest)))
  (LocalVariables|SetRegistrationRequestObject _returnvalue)
  (Class|VaRestJsonObject|SetStringField (LocalVariables|GetRegistrationRequestObject) "accountname" (Utilities|String|ToString(Text) (Class|EditableTextBox|GetText (Variables|/Game/Blueprints/widgets/mutagenLogin_WB.mutagenLogin_WB_C|GetregistrationUserNameTextbox (Variables|ReferencesBP|GetLoginWidgetRef_BP)))))
  (Class|VaRestJsonObject|SetStringField (LocalVariables|GetRegistrationRequestObject) "accountemail" (Utilities|String|ToString(Text) (Class|EditableTextBox|GetText (Variables|/Game/Blueprints/widgets/mutagenLogin_WB.mutagenLogin_WB_C|GetRegistrationEmailTextBox (Variables|ReferencesBP|GetLoginWidgetRef_BP)))))
  (Class|VaRestJsonObject|SetStringField (LocalVariables|GetRegistrationRequestObject) "accountpassword" (Utilities|String|ToString(Text) (Class|EditableTextBox|GetText (Variables|/Game/Blueprints/widgets/mutagenLogin_WB.mutagenLogin_WB_C|GetregistrationPasswordTextBox (Variables|ReferencesBP|GetLoginWidgetRef_BP)))))
  (Class|VaRestJsonObject|SetStringField (LocalVariables|GetRegistrationRequestObject) "accountsecurityquestion" (Class|ComboBoxString|GetSelectedOption (Variables|/Game/Blueprints/widgets/mutagenLogin_WB.mutagenLogin_WB_C|GetsecurityQuestionsComboBox (Variables|ReferencesBP|GetLoginWidgetRef_BP))))
  (Class|VaRestJsonObject|SetStringField (LocalVariables|GetRegistrationRequestObject) "accountsecurityanswer" (Utilities|String|ToString(Text) (Class|EditableTextBox|GetText (Variables|/Game/Blueprints/widgets/mutagenLogin_WB.mutagenLogin_WB_C|GetregistrationSecurityAnswer (Variables|ReferencesBP|GetLoginWidgetRef_BP)))))
  (for _index (range 0 8)
    ;[0 0.1364 1] Create a random 8 letter string
    (LocalVariables|SetRandomAccountString (Utilities|String|Append (Utilities|Array|Get(acopy) (LocalVariables|GetAlphabetArray) (Math|Random|RandomInteger 52)) (LocalVariables|GetRandomAccountString)))
    ;[0 0.1364 1] Create a random number between 0 & 99999
    (LocalVariables|SetRandomAccountnumber (Utilities|String|ToString(Integer) (Math|Random|RandomInteger 99999))))
  ;[0 0.1364 1] Create the random AccountUniqueId by combining the random string and number
  (bind _output_get (LocalVariables|SetAccountUniqueID (Utilities|String|Append (LocalVariables|GetRandomAccountnumber) (LocalVariables|GetRandomAccountString))))
  ;[0 0.1364 1] Turn the random AccountUniqueID into a char array
  (bind _output_get_2 (LocalVariables|SetUniqueCharArray (Utilities|String|GetCharacterArrayfromString _output_get)))
  ;[0 0.1364 1] Loop through the char array and pick a char at random
  ; Then add it back to the AccountUniqueID string
  ; So now we have a completly random Unique ID with a mixture of letters and numbers
  (for _index_2 (range 0 5)
    (bind _output_get_3 (LocalVariables|SetAccountUniqueID (Utilities|String|Append (LocalVariables|GetAccountUniqueID) (Utilities|Array|Get(acopy) _output_get_2 (Math|Random|RandomInteger (Utilities|Array|Length _output_get_2)))))))
  (Class|VaRestJsonObject|SetStringField (LocalVariables|GetRegistrationRequestObject) "accountuniqueID" _output_get_3)
  (CallFunction|CallPhpScript (Variables|VaRest|GetSentRequest) "registration"))

(fn SetUpLoginWidgetRef
  (bind _asmutagen_login_wb (Utilities|Casting|CastTomutagenLogin_WB (Variables|RefC++|GetLoginWidgetRef))
    (:then
      (Variables|ReferencesBP|SetLoginWidgetRef_BP _asmutagen_login_wb))
    (:CastFailed
      (Development|PrintString "Hello"))))

(fn CallPhpScript
  (params (Request :type Va%20Rest%20Request%20JSON%20Object%20Reference) (PhpScriptName :type String))
  (bind _hostname (Variables|Default|GetHostName))
  (bind _returnvalue (Utilities|String|EndsWith _hostname "/"))
  (bind _returnvalue_2 (Utilities|String|Append _hostname "/"))
  (bind _returnvalue_3 (select _returnvalue _hostname _returnvalue_2))
  (bind _returnvalue_4 (Utilities|String|Append _returnvalue_3 PhpScriptName))
  (bind _returnvalue_5 (Utilities|String|Append _returnvalue_4 ".php"))
  (Development|PrintString _returnvalue_5)
  (Class|VaRestRequestJSON|ProcessURL Request _returnvalue_5))

(fn OnResponceRegistration
  (bind _returnvalue (Class|VaRestRequestJSON|GetResponseObject (Variables|VaRest|GetSentRequest)))
  (LocalVariables|SetRegistrationResponceObject _returnvalue)
  (if (Utilities|Enum|Equal(Enum) (Class|VaRestJsonObject|GetStringField _returnvalue "status") "ok")
    (CallFunction|ClearUserInput)
    (Default|DisplayRegistrationErrorMessage (Variables|ReferencesBP|GetLoginWidgetRef_BP) "Registration Successful")
    (Utilities|Time|SetTimerbyFunctionName 0 "GoToActivationPanel" 1.0)
    (else
      (Default|DisplayRegistrationErrorMessage (Variables|ReferencesBP|GetLoginWidgetRef_BP) (Utilities|Text|ToText(String) (Class|VaRestJsonObject|GetStringField _returnvalue "status"))))))

(fn ClearUserInput
  (Rendering|Components|TextRender|SetText (Variables|/Game/Blueprints/widgets/mutagenLogin_WB.mutagenLogin_WB_C|GetregistrationUserNameTextbox (Variables|ReferencesBP|GetLoginWidgetRef_BP)) "")
  (Rendering|Components|TextRender|SetText (Variables|/Game/Blueprints/widgets/mutagenLogin_WB.mutagenLogin_WB_C|GetRegistrationEmailTextBox (Variables|ReferencesBP|GetLoginWidgetRef_BP)) "")
  (Rendering|Components|TextRender|SetText (Variables|/Game/Blueprints/widgets/mutagenLogin_WB.mutagenLogin_WB_C|GetregistrationPasswordTextBox (Variables|ReferencesBP|GetLoginWidgetRef_BP)) "")
  (Rendering|Components|TextRender|SetText (Variables|/Game/Blueprints/widgets/mutagenLogin_WB.mutagenLogin_WB_C|GetregistrationRepeatPasswordTextBox (Variables|ReferencesBP|GetLoginWidgetRef_BP)) "")
  (Rendering|Components|TextRender|SetText (Variables|/Game/Blueprints/widgets/mutagenLogin_WB.mutagenLogin_WB_C|GetregistrationSecurityAnswer (Variables|ReferencesBP|GetLoginWidgetRef_BP)) ""))

(fn GotoActivationPanel
  (Default|GotoActivationPanelfromRegistration (Variables|ReferencesBP|GetLoginWidgetRef_BP)))

(fn CreateActivationRequest
  (bind _loginwidgetref_bp (Variables|ReferencesBP|GetLoginWidgetRef_BP))
  (bind _activationaccountuniqueidbox (Variables|/Game/Blueprints/widgets/mutagenLogin_WB.mutagenLogin_WB_C|GetactivationAccountUniqueIDBox _loginwidgetref_bp))
  (bind _returnvalue (Class|VaRestRequestJSON|GetRequestObject (Variables|VaRest|GetSentRequest)))
  (LocalVariables|SetActivationRequestObject _returnvalue)
  (Class|VaRestJsonObject|SetStringField (LocalVariables|GetActivationRequestObject) "accountUniqueID" (Utilities|String|ToString(Text) (Class|EditableTextBox|GetText _activationaccountuniqueidbox)))
  (Rendering|Components|TextRender|SetText _activationaccountuniqueidbox "")
  (CallFunction|CallPhpScript (Variables|VaRest|GetSentRequest) "activationRequest"))

(fn OnResponceActivation
  (bind _returnvalue (Class|VaRestRequestJSON|GetResponseObject (Variables|VaRest|GetSentRequest)))
  (LocalVariables|SetActivationResponceObject _returnvalue)
  (if (Utilities|Enum|Equal(Enum) (Class|VaRestJsonObject|GetStringField _returnvalue "status") "account found")
    (Default|DisplayActivationErrorMessage (Variables|ReferencesBP|GetLoginWidgetRef_BP) "Account Activated")
    (Utilities|Time|SetTimerbyFunctionName 0 "GoToLoginPanelFromActivation" 1.0)
    (else
      (Default|DisplayActivationErrorMessage (Variables|ReferencesBP|GetLoginWidgetRef_BP) (Utilities|Text|ToText(String) (Class|VaRestJsonObject|GetStringField _returnvalue "status"))))))

(fn GotoLoginPanelfromActivation
  (Default|GotoLoginPanelfromActivation (Variables|ReferencesBP|GetLoginWidgetRef_BP)))

(fn CreateLoginRequest
  (bind _loginwidgetref_bp (Variables|ReferencesBP|GetLoginWidgetRef_BP))
  (bind _returnvalue (Class|VaRestRequestJSON|GetRequestObject (Variables|VaRest|GetSentRequest)))
  (LocalVariables|SetLoginRequestObject _returnvalue)
  (Class|VaRestJsonObject|SetStringField (LocalVariables|GetLoginRequestObject) "login" (Utilities|String|ToString(Text) (Class|EditableTextBox|GetText (Variables|/Game/Blueprints/widgets/mutagenLogin_WB.mutagenLogin_WB_C|GetUsername-Input (Variables|ReferencesBP|GetLoginWidgetRef_BP)))))
  (Class|VaRestJsonObject|SetStringField (LocalVariables|GetLoginRequestObject) "password" (Utilities|String|ToString(Text) (Class|EditableTextBox|GetText (Variables|/Game/Blueprints/widgets/mutagenLogin_WB.mutagenLogin_WB_C|GetPassword-Input (Variables|ReferencesBP|GetLoginWidgetRef_BP)))))
  (Rendering|Components|TextRender|SetText (Variables|/Game/Blueprints/widgets/mutagenLogin_WB.mutagenLogin_WB_C|GetPassword-Input _loginwidgetref_bp) "")
  (Rendering|Components|TextRender|SetText (Variables|/Game/Blueprints/widgets/mutagenLogin_WB.mutagenLogin_WB_C|GetUsername-Input _loginwidgetref_bp) "")
  (CallFunction|CallPhpScript (Variables|VaRest|GetSentRequest) "login"))

(fn OnResponceLogin
  (bind _returnvalue (Class|VaRestRequestJSON|GetResponseObject (Variables|VaRest|GetSentRequest)))
  (LocalVariables|SetLoginResponceObject _returnvalue)
  (if (Utilities|Enum|Equal(Enum) (Class|VaRestJsonObject|GetStringField _returnvalue "status") "ok")
    (Default|DisplayLoginErrorMessage (Variables|ReferencesBP|GetLoginWidgetRef_BP) "Login Sucessful")
    (Variables|Default|SetMysessionKey (Class|VaRestJsonObject|GetStringField (LocalVariables|GetLoginResponceObject) "sessionKey"))
    (Variables|Default|SetMyUserID (Math|Float|Floor (Class|VaRestJsonObject|GetNumberField (LocalVariables|GetLoginResponceObject) "userid")))
    (CallFunction|SendRequestEvent "NewEnumerator3")
    (else
      (Default|DisplayLoginErrorMessage (Variables|ReferencesBP|GetLoginWidgetRef_BP) (Utilities|Text|ToText(String) (Class|VaRestJsonObject|GetStringField _returnvalue "status"))))))

(fn CreateCheckforCharactersRequest
  (bind _returnvalue (Class|VaRestRequestJSON|GetRequestObject (Variables|VaRest|GetSentRequest)))
  (LocalVariables|SetCharacterCheckRequestObject _returnvalue)
  (Class|VaRestJsonObject|SetStringField (LocalVariables|GetCharacterCheckRequestObject) "sessionkey" (Variables|Default|GetMysessionKey))
  (Class|VaRestJsonObject|SetNumberField (LocalVariables|GetCharacterCheckRequestObject) "userid" (Math|Conversions|ToFloat(Integer) (Variables|Default|GetMyUserID)))
  (CallFunction|CallPhpScript (Variables|VaRest|GetSentRequest) "checkCharacters"))

(fn OnResponceCheckCharacters
  (bind _returnvalue (Class|VaRestRequestJSON|GetResponseObject (Variables|VaRest|GetSentRequest)))
  (LocalVariables|SetCheckCharactersResponceObject _returnvalue))